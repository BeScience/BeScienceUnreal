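; BP_ElecticPipeLine is a connectable electric line segment with two sphere ends that carries power and polarity between actors.
; Tick pulls the ends together with forces whenever they exceed a set distance.
; Overlaps record new actors, stop that end's physics and snap the other component on; side 2 also notifies lines and batteries.
; OnElectron stores the values and recursively forwards them to recorded lines whose power differs.
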(event `self.ReceiveTick`
  (params (DeltaSeconds :type "Float (single-precision)"))
  (bind _spherecolision_side1 (`self.SphereColision_Side1`))
  (bind _spherecolision_side2 (`self.SphereColision_Side2`))
  (bind _power (`self.power`))
  (bind _returnvalue (`SceneComponent.K2_GetComponentLocation` _spherecolision_side2))
  (bind _returnvalue_2 (`SceneComponent.K2_GetComponentLocation` _spherecolision_side1))
  (bind _returnvalue_3 (- _returnvalue _returnvalue_2))
  (if (> (`KismetMathLibrary.VSize` _returnvalue_3) 200.0)
    (set `self.power` 1.0)
    (`PrimitiveComponent.AddForce` _spherecolision_side1 (* _returnvalue_3 _power) "None" false)
    (`PrimitiveComponent.AddForce` _spherecolision_side2 (* (- _returnvalue_2 _returnvalue) _power) "None" false)
    (else
      (set `self.power` 0.0))))

(event `self.SphereColision_Side1.OnComponentBeginOverlap`
  (params (OverlappedComponent :type "PrimitiveComponent Object Reference") (OtherActor :type "Actor Object Reference") (OtherComp :type "PrimitiveComponent Object Reference") (OtherBodyIndex :type Integer) (bFromSweep :type Boolean) (SweepResult :type "HitResult Structure (by ref)"))
  (if (== (`KismetArrayLibrary.Array_Find` (`self.Other Actor`) OtherActor) -1)
    (if (not (== OtherActor self))
      (`KismetArrayLibrary.Array_Add` (`self.Other Actor`) OtherActor)
      (`PrimitiveComponent.SetSimulatePhysics` OverlappedComponent false)
      (`SceneComponent.K2_AttachToComponent` OtherComp OverlappedComponent "None" "SnapToTarget" "SnapToTarget" "SnapToTarget" true))))

(event `self.SphereColision_Side2.OnComponentBeginOverlap`
  (params (OverlappedComponent :type "PrimitiveComponent Object Reference") (OtherActor :type "Actor Object Reference") (OtherComp :type "PrimitiveComponent Object Reference") (OtherBodyIndex :type Integer) (bFromSweep :type Boolean) (SweepResult :type "HitResult Structure (by ref)"))
  (if (== (`KismetArrayLibrary.Array_Find` (`self.Other Actor`) OtherActor) -1)
    (if (not (== OtherActor self))
      (`KismetArrayLibrary.Array_Add` (`self.Other Actor`) OtherActor)
      (`PrimitiveComponent.SetSimulatePhysics` OverlappedComponent false)
      (`SceneComponent.K2_AttachToComponent` OtherComp OverlappedComponent "None" "SnapToTarget" "SnapToTarget" "SnapToTarget" true)
      (`|ExecutionSequence`
        (:`then_0`
          (bind _asbp_electic_pipe_line (cast `/Game/Kyoulee/BluePrints/Electricity/BP_ElecticPipeLine` OtherActor))
          (`self.OnElectron` _asbp_electic_pipe_line (`self.polarity`) (`self.ElecPower`)))
        (:`then_1`
          (bind _asbp_electic_pipe_bettery (cast `/Game/Kyoulee/BluePrints/Electricity/BP_ElecticPipeBettery` OtherActor))
          (`/Game/Kyoulee/BluePrints/Electricity/BP_ElecticPipeBettery.SendElectronic` _asbp_electic_pipe_bettery))
        (:`then_2`
          (cast `/Game/Kyoulee/BluePrints/Electricity/BP_ElecticLight` OtherActor))))))

(event `OnElectron`
  (params (otherPolarity :type Boolean) (otherElecPower :type Integer))
  (set `self.ElecPower` otherElecPower)
  (set `self.polarity` otherPolarity)
  (for _array_element (`self.Other Actor`)
    (`|ExecutionSequence`
      (:`then_0`
        (bind _asbp_electic_pipe_line (cast `/Game/Kyoulee/BluePrints/Electricity/BP_ElecticPipeLine` _array_element))
        (if (!= (`/Game/Kyoulee/BluePrints/Electricity/BP_ElecticPipeLine.ElecPower` _asbp_electic_pipe_line) otherElecPower)
          (`self.OnElectron` _asbp_electic_pipe_line otherPolarity otherElecPower))))))

(fn `UserConstructionScript`)