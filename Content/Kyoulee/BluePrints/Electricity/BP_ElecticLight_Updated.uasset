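; BP_ElecticLight_Updated is an electric light whose point light brightness follows the voltage it receives.
; It extends a parent electricity Blueprint, overriding Update Volt to scale PointLight intensity linearly with Volt and print the result.
; Its OnGrabComponent override calls the parent, then detaches the Capsule while keeping its world transform.
; An older TurnOn-based intensity setter remains in the EventGraph but never runs.
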(fn `OnGrabComponent`
  (params (Component :type "PrimitiveComponent Object Reference"))
  (`parent.OnGrabComponent` Component)
  (`SceneComponent.K2_DetachFromComponent` (`self.Capsule`) "KeepWorld" "KeepWorld" "KeepWorld" true))

(fn `Update Volt`
  (bind _returnvalue (* 10000.0 (`self.Volt`)))
  (`parent.Update Volt`)
  (`LightComponent.SetIntensity` (`self.PointLight`) _returnvalue)
  (`KismetSystemLibrary.PrintString` (`KismetStringLibrary.Concat_StrStr` "light volt" (`KismetStringLibrary.Conv_DoubleToString` _returnvalue))))

(fn `UserConstructionScript`)