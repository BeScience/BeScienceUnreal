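; BP_ElecticPipeStreat3 is an electric pipe piece with two sphere-collision ends that act as a loose tether and snap-on connectors.
; Each Tick, when the ends are more than a fixed distance apart in relative space, it adds opposing forces along their offset to pull them together.
; On overlap, an end stops simulating physics and the overlapping component is attached to it with location, rotation and scale snapped.
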(event `self.ReceiveTick`
  (params (DeltaSeconds :type "Float (single-precision)"))
  (bind _spherecolision_side1 (`self.SphereColision_Side1`))
  (bind _spherecolision_side2 (`self.SphereColision_Side2`))
  (bind _power (`self.power`))
  (bind _relativelocation (`SceneComponent.RelativeLocation` _spherecolision_side1))
  (bind _relativelocation_2 (`SceneComponent.RelativeLocation` _spherecolision_side2))
  (bind _returnvalue (- _relativelocation_2 _relativelocation))
  (if (> (`KismetMathLibrary.VSize` _returnvalue) 200.0)
    (set `self.power` 1.0)
    (`PrimitiveComponent.AddForce` _spherecolision_side1 (* _returnvalue _power) "None" false)
    (`PrimitiveComponent.AddForce` _spherecolision_side2 (* (- _relativelocation _relativelocation_2) _power) "None" false)
    (else
      (set `self.power` 0.0))))

(event `self.SphereColision_Side1.OnComponentBeginOverlap`
  (params (OverlappedComponent :type "PrimitiveComponent Object Reference") (OtherActor :type "Actor Object Reference") (OtherComp :type "PrimitiveComponent Object Reference") (OtherBodyIndex :type Integer) (bFromSweep :type Boolean) (SweepResult :type "HitResult Structure (by ref)"))
  (`PrimitiveComponent.SetSimulatePhysics` OverlappedComponent false)
  (`SceneComponent.K2_AttachToComponent` OtherComp OverlappedComponent "None" "SnapToTarget" "SnapToTarget" "SnapToTarget" true))

(event `self.SphereColision_Side2.OnComponentBeginOverlap`
  (params (OverlappedComponent :type "PrimitiveComponent Object Reference") (OtherActor :type "Actor Object Reference") (OtherComp :type "PrimitiveComponent Object Reference") (OtherBodyIndex :type Integer) (bFromSweep :type Boolean) (SweepResult :type "HitResult Structure (by ref)"))
  (`PrimitiveComponent.SetSimulatePhysics` OverlappedComponent false)
  (`SceneComponent.K2_AttachToComponent` OtherComp OverlappedComponent "None" "SnapToTarget" "SnapToTarget" "SnapToTarget" true))

(fn `UserConstructionScript`)