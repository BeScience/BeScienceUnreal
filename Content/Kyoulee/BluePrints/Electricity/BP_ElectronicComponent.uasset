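; Electronic component Blueprint that tracks connections to other components and derives its own voltage from them.
; Connecting sorts the other component into plus or minus lists by voltage sign, with zero counted as minus, and disconnecting removes it from both.
; CalculateVolt requires both lists non-empty and sets Volt to Min(MaxVolt, Abs(MinVolt)).
; The minus-side loop writes into MaxVolt instead of MinVolt, so MinVolt stays zero.
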(event `ConnectElectronic`
  (params (NewConnect :type "/Game/Kyoulee/BluePrints/Electricity/BP_ElectronicBase Object Reference"))
  (if (> (`/Game/Kyoulee/BluePrints/Electricity/BP_ElectronicBase.Volt` NewConnect) 0.0)
    (`KismetArrayLibrary.Array_Add` (`self.PlusConnectedOthers`) NewConnect)
    (else
      (`KismetArrayLibrary.Array_Add` (`self.MinusConnectedOthers`) NewConnect))))

(event `CalculateVolt`
  (if (> (`KismetArrayLibrary.Array_Length` (`self.PlusConnectedOthers`)) 0)
    (if (> (`KismetArrayLibrary.Array_Length` (`self.MinusConnectedOthers`)) 0)
      (`|ExecutionSequence`
        (:`then_0`
          (set `self.MaxVolt` 0.0)
          (for _array_element (`self.PlusConnectedOthers`)
            (bind _volt (`/Game/Kyoulee/BluePrints/Electricity/BP_ElectronicBase.Volt` _array_element))
            (if (> _volt (`self.MaxVolt`))
              (set `self.MaxVolt` _volt))))
        (:`then_1`
          (set `self.MinVolt` 0.0)
          (for _array_element_2 (`self.MinusConnectedOthers`)
            (bind _volt_2 (`/Game/Kyoulee/BluePrints/Electricity/BP_ElectronicBase.Volt` _array_element_2))
            (if (< _volt_2 (`self.MinVolt`))
              (set `self.MaxVolt` _volt_2))))
        (:`then_2`
          (set `self.Volt` (`KismetMathLibrary.FMin` (`self.MaxVolt`) (`KismetMathLibrary.Abs` (`self.MinVolt`)))))))))

(event `LeftdisconnectEletronic`
  (params (Disconnect :type "/Game/Kyoulee/BluePrints/Electricity/BP_ElectronicBase Object Reference"))
  (`|ExecutionSequence`
    (:`then_0`
      (`KismetArrayLibrary.Array_RemoveItem` (`self.PlusConnectedOthers`) Disconnect))
    (:`then_1`
      (`KismetArrayLibrary.Array_RemoveItem` (`self.MinusConnectedOthers`) Disconnect))))