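; BP_BetteryConnectBox is an electricity socket that lights its connected lights when a BP_ElecticPipeBettery is placed in it.
; Box overlap stores the battery, then sets each ConnectLight point light's intensity high if a forward-vector dot product shows both face the same general way.
; When that stored battery leaves the box, the lights drop to zero intensity.
; The battery reference has an OnRep function, which is empty.
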(event `self.Box.OnComponentBeginOverlap`
  (params (OverlappedComponent :type "PrimitiveComponent Object Reference") (OtherActor :type "Actor Object Reference") (OtherComp :type "PrimitiveComponent Object Reference") (OtherBodyIndex :type Integer) (bFromSweep :type Boolean) (SweepResult :type "HitResult Structure (by ref)"))
  (bind _asbp_electic_pipe_bettery (cast `/Game/Kyoulee/BluePrints/Electricity/BP_ElecticPipeBettery` OtherActor))
  (set `self.As BP Electic Pipe Bettery` _asbp_electic_pipe_bettery)
  (if (> (`KismetMathLibrary.Dot_VectorVector` (`self.GetActorForwardVector` _asbp_electic_pipe_bettery) (`self.GetActorForwardVector` self)) 0.0)
    (bind (_arrayindex _arrayelement) (`/Engine/EditorBlueprintResources/StandardMacros.ReverseForEachLoop` (`self.ConnectLight`))
      (:`LoopBody`
        (`LightComponent.SetIntensity` (`/Game/Kyoulee/BluePrints/Electricity/BP_ElecticLight.PointLight` _arrayelement) 2000.0)))))

(event `self.Box.OnComponentEndOverlap`
  (params (OverlappedComponent :type "PrimitiveComponent Object Reference") (OtherActor :type "Actor Object Reference") (OtherComp :type "PrimitiveComponent Object Reference") (OtherBodyIndex :type Integer))
  (bind _asbp_electic_pipe_bettery (cast `/Game/Kyoulee/BluePrints/Electricity/BP_ElecticPipeBettery` OtherActor))
  (if (== _asbp_electic_pipe_bettery (`self.As BP Electic Pipe Bettery`))
    (bind (_arrayindex _arrayelement) (`/Engine/EditorBlueprintResources/StandardMacros.ReverseForEachLoop` (`self.ConnectLight`))
      (:`LoopBody`
        (`LightComponent.SetIntensity` (`/Game/Kyoulee/BluePrints/Electricity/BP_ElecticLight.PointLight` _arrayelement) 0.0)))))

(fn `OnRep_As BP Electic Pipe Bettery`)

(fn `UserConstructionScript`)