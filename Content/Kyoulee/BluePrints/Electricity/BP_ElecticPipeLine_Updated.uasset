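; Electric pipe line actor with two sphere-collision ends that link it to other BP_ElectronicBase actors in a circuit.
; Overlap on either end connects the other electronic component and updates voltage, while end overlap disconnects it without an explicit voltage update here.
; Grabbing a component runs the parent logic, then detaches it in world space.
; Battery-polarity and spring-force logic between the ends is present but never runs.
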(event `self.ReceiveTick`
  (params (DeltaSeconds :type "Float (single-precision)")))

(event `self.SphereColision_Side1.OnComponentBeginOverlap`
  (params (OverlappedComponent :type "PrimitiveComponent Object Reference") (OtherActor :type "Actor Object Reference") (OtherComp :type "PrimitiveComponent Object Reference") (OtherBodyIndex :type Integer) (bFromSweep :type Boolean) (SweepResult :type "HitResult Structure (by ref)"))
  (bind _asbp_electronic_base (cast `/Game/Kyoulee/BluePrints/Electricity/BP_ElectronicBase` OtherActor))
  (if (not (== self _asbp_electronic_base))
    (`self.Connect Other Electronic` OverlappedComponent OtherComp _asbp_electronic_base)
    (`self.Update Volt`)))

(event `self.SphereColision_Side2.OnComponentBeginOverlap`
  (params (OverlappedComponent :type "PrimitiveComponent Object Reference") (OtherActor :type "Actor Object Reference") (OtherComp :type "PrimitiveComponent Object Reference") (OtherBodyIndex :type Integer) (bFromSweep :type Boolean) (SweepResult :type "HitResult Structure (by ref)"))
  (bind _asbp_electronic_base (cast `/Game/Kyoulee/BluePrints/Electricity/BP_ElectronicBase` OtherActor))
  (if (not (== self _asbp_electronic_base))
    (`self.Connect Other Electronic` OverlappedComponent OtherComp _asbp_electronic_base)
    (`self.Update Volt`)))

(event `self.SphereColision_Side2.OnComponentEndOverlap`
  (params (OverlappedComponent :type "PrimitiveComponent Object Reference") (OtherActor :type "Actor Object Reference") (OtherComp :type "PrimitiveComponent Object Reference") (OtherBodyIndex :type Integer))
  (bind _asbp_electronic_base (cast `/Game/Kyoulee/BluePrints/Electricity/BP_ElectronicBase` OtherActor))
  (if (not (== self _asbp_electronic_base))
    (`self.DisconnectOtherElectronic` OverlappedComponent OtherComp _asbp_electronic_base)))

(event `self.SphereColision_Side1.OnComponentEndOverlap`
  (params (OverlappedComponent :type "PrimitiveComponent Object Reference") (OtherActor :type "Actor Object Reference") (OtherComp :type "PrimitiveComponent Object Reference") (OtherBodyIndex :type Integer))
  (bind _asbp_electronic_base (cast `/Game/Kyoulee/BluePrints/Electricity/BP_ElectronicBase` OtherActor))
  (if (not (== self _asbp_electronic_base))
    (`self.DisconnectOtherElectronic` OverlappedComponent OtherComp _asbp_electronic_base)))

(fn `OnGrabComponent`
  (params (Component :type "PrimitiveComponent Object Reference"))
  (`parent.OnGrabComponent` Component)
  (`SceneComponent.K2_DetachFromComponent` Component "KeepWorld" "KeepWorld" "KeepWorld" true))

(fn `UserConstructionScript`)