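; BP_Door is a sliding double door that opens and closes with the on/off state of a linked Light in the electricity setup.
; On BeginPlay it binds to the Light's OnLightSetting event and copies TurnOn into Opened, which OpenDoor and CloseDoor events can also set.
; Tick moves DoorMove toward MaxMove or zero at MoveSpeed, offsetting the Left and Right parts in opposite directions along relative X.
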(event `self.ReceiveBeginPlay`
  (add `/Game/Kyoulee/BluePrints/Electricity/BP_ElecticLight.OnLightSetting` (`self.light`) (delegate `OnLightEvent`)))

(event `OnLightEvent`
  (if (`/Game/Kyoulee/BluePrints/Electricity/BP_ElecticLight.turnOn` (`self.light`))
    (set `self.bOpened` true)
    (else
      (set `self.bOpened` false))))

(event `self.ReceiveTick`
  (params (DeltaSeconds :type "Float (single-precision)"))
  (bind _returnvalue (* DeltaSeconds (`self.MoveSpeed`)))
  (if (`self.bOpened`)
    (if (< (`self.DoorMove`) (`self.MaxMove`))
      (set `self.DoorMove` (+ (`self.DoorMove`) _returnvalue))
      (`SceneComponent.K2_SetRelativeLocation` (`self.Left`) (`KismetMathLibrary.MakeVector` (`self.DoorMove`)) false false :!label _label)
      (`SceneComponent.K2_SetRelativeLocation` (`self.Right`) (`KismetMathLibrary.MakeVector` (* (`self.DoorMove`) -1.0)) false false))
    (elif (> (`self.DoorMove`) 0.0)
      (set `self.DoorMove` (- (`self.DoorMove`) _returnvalue))
      (goto _label))))

(event `OpenDoor`
  (set `self.bOpened` true))

(event `CloseDoor`
  (set `self.bOpened` false))

(fn `UserConstructionScript`)