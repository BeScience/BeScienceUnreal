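; BP_Login_UI is a trigger actor that shows the login HUD while the player character is inside its Sphere.
; On first entry it creates and caches WBP_Login_HUD, focuses it in Game and UI input mode and shows the cursor.
; Later entries only make the cached widget visible, without restoring cursor or focus.
; Leaving collapses the widget and hides the cursor, but leaves the input mode unchanged.
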(event `self.ReceiveBeginPlay`)

(event `self.Sphere.OnComponentBeginOverlap`
  (params (OverlappedComponent :type "PrimitiveComponent Object Reference") (OtherActor :type "Actor Object Reference") (OtherComp :type "PrimitiveComponent Object Reference") (OtherBodyIndex :type Integer) (bFromSweep :type Boolean) (SweepResult :type "HitResult Structure (by ref)"))
  (bind _returnvalue (`GameplayStatics.GetPlayerController` 0))
  (if (== OtherActor (`GameplayStatics.GetPlayerCharacter` 0))
    ;[1 1 1] 입력 widget
    (bind _loginwidget (`self.LoginWidget`)
      (:`then`
        (`Widget.SetVisibility` _loginwidget "Visible"))
      (:`else`
        (bind _returnvalue_2 (`|CreateWidget` "/Game/Kyoulee/BluePrints/Ticket/Widgets/WBP_Login_HUD.WBP_Login_HUD_C"))
        (bind _output_get (set `self.LoginWidget` _returnvalue_2))
        (`UserWidget.AddToViewport` _output_get 0)
        (`WidgetBlueprintLibrary.SetInputMode_GameAndUIEx` _returnvalue _returnvalue_2)
        (set `PlayerController.bShowMouseCursor` true _returnvalue)))))

(event `self.Sphere.OnComponentEndOverlap`
  (params (OverlappedComponent :type "PrimitiveComponent Object Reference") (OtherActor :type "Actor Object Reference") (OtherComp :type "PrimitiveComponent Object Reference") (OtherBodyIndex :type Integer))
  (if (== OtherActor (`GameplayStatics.GetPlayerCharacter` 0))
    ;[1 1 1] widget 감추기
    (`Widget.SetVisibility` (`self.LoginWidget`) "Collapsed")
    (set `PlayerController.bShowMouseCursor` false (`GameplayStatics.GetPlayerController` 0))))

(fn `UserConstructionScript`)