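; Game menu component that toggles the WBP_GameMenu widget when T or Escape is pressed.
; The first press creates the widget and adds it to the viewport, and later presses switch it between visible and collapsed rather than recreating it.
; Player 0's mouse cursor is shown while the menu is open and hidden when it collapses.
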(event `Key|T`
  (params (Key :type "Key Structure"))
  (:`Pressed`
    (bind _menuwidget (`self.MenuWidget` :!label _label)
      (:`then`
        (if (`|EnumEquality` (`Widget.GetVisibility` _menuwidget) "Collapsed")
          (`Widget.SetVisibility` (`self.MenuWidget`) "Visible")
          (set `PlayerController.bShowMouseCursor` true (`GameplayStatics.GetPlayerController` 0) :!label _label_2)
          (`Widget.ForceVolatile` (stale _output_get) false)
          (else
            (`Widget.SetVisibility` (`self.MenuWidget`) "Collapsed")
            (set `PlayerController.bShowMouseCursor` false (`GameplayStatics.GetPlayerController` 0)))))
      (:`else`
        (bind _returnvalue (`|CreateWidget` "/Game/Kyoulee/WidGets/GameWidget/WBP_GameMenu.WBP_GameMenu_C"))
        (bind _output_get (set `self.MenuWidget` _returnvalue))
        (`UserWidget.AddToViewport` _output_get 0)
        (goto _label_2)))))

(event `Key|Escape`
  (params (Key :type "Key Structure"))
  (:`Pressed`
    (goto _label)))