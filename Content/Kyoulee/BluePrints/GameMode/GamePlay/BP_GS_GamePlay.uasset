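; Game state for gameplay that runs a replicated countdown to match start and shows it on screen.
; A player connection notification updates the player count and, while it is at or below the required minimum, seeds the countdown once.
; The countdown's RepNotify refreshes every WBP_MatchStartCountDown widget, and on the server re-triggers itself through a one-second decrement event.
; At zero the server only prints "Start Match".
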(event `/Game/Kyoulee/BluePrints/Interfaces/BPI_GameState.Notify_PlayerConnection`
  (bind _returnvalue (`GameplayStatics.GetNumPlayerStates`))
  (set `self.CurrentAmountOfPlayers` _returnvalue)
  (if (<= _returnvalue (`self.MinimumRequiredPlayers`))
    (`/Engine/EditorBlueprintResources/StandardMacros.DoOnce` false
      (:`Completed`
        (set `self.MatchStart_Countdown` 15)))))

(event `Match Coundown`
  (`KismetSystemLibrary.Delay` 1.0)
  (set `self.MatchStart_Countdown` (- (`self.MatchStart_Countdown`) 1)))

(fn `OnRep_MatchStart_Countdown`
  (`self.Update_MatchStartCountdownWidget`)
  ;[1 1 1] authority 서버만
  ; Remote 클라이언트만
  (`/Engine/EditorBlueprintResources/ActorMacros.Switch Has Authority`
    (:`Authority`
      (if (<= (`self.MatchStart_Countdown`) 0)
        (`KismetSystemLibrary.PrintString` "Start Match")
        (else
          (`self.Match Coundown`))))))

(fn `Update_MatchStartCountdownWidget`
  (bind _foundwidgets (`WidgetBlueprintLibrary.GetAllWidgetsOfClass` "/Game/Kyoulee/WidGets/GameWidget/WBP_MatchStartCountDown.WBP_MatchStartCountDown_C" false))
  (for _array_element _foundwidgets
    (`/Game/Kyoulee/WidGets/GameWidget/WBP_MatchStartCountDown.Update_Widget` _array_element (`self.MatchStart_Countdown`))))

(fn `UserConstructionScript`
  (`parent.UserConstructionScript`))