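; BP_GM_Test_GamePlay is a test gameplay Game Mode that reports player connection changes.
; Both PostLogin and OnLogout call NotifyPlayerConnectionMessage on the Game State, leaving the message handling to that class.
; BeginPlay, Tick and the construction script add no logic of their own.
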(event `self.K2_PostLogin`
  (params (NewPlayer :type "PlayerController Object Reference"))
  ;[1 1 1] 현재 플레이어 뷰 포트 설정
  (message `/Game/Kyoulee/BluePrints/Interfaces/BPI_GameState.Notify_PlayerConnection` (`GameplayStatics.GetGameState`)))

(event `self.K2_OnLogout`
  (params (ExitingController :type "Controller Object Reference"))
  (message `/Game/Kyoulee/BluePrints/Interfaces/BPI_GameState.Notify_PlayerConnection` (`GameplayStatics.GetGameState`)))

(fn `UserConstructionScript`
  (`parent.UserConstructionScript`))