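; Test character Blueprint that lets the player pick up, carry and release objects through a Physics Handle.
; Pressing G toggles the grab, using a debug-drawn Visibility line trace from the capsule toward the follow camera's forward direction and grabbing the hit component.
; While holding, Tick moves the handle target to a short, fixed distance from the capsule along the camera's forward vector.
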(event `self.ReceiveTick`
  (params (DeltaSeconds :type "Float (single-precision)"))
  ;[1 1 1] Pick object
  (if (`self.GrapObject`)
    (`PhysicsHandleComponent.SetTargetLocation` (`self.PhysicsHandle`) (+ (`SceneComponent.K2_GetComponentLocation` (`self.CapsuleComponent`)) (* (`KismetMathLibrary.GetForwardVector` (`SceneComponent.K2_GetComponentRotation` (`self.FollowCamera`))) 150.0)))))

(event `Key|G`
  (params (Key :type "Key Structure"))
  (bind _capsulecomponent (`self.CapsuleComponent`))
  ;[1 1 1] Grap object
  (:`Pressed`
    (if (`self.GrapObject`)
      (if (`self.GrapObject`)
        (`PhysicsHandleComponent.ReleaseComponent` (`self.PhysicsHandle`))
        (set `self.GrapObject` false))
      (else
        (bind (_outhit _returnvalue) (`KismetSystemLibrary.LineTraceSingle` :`Start` (+ (`SceneComponent.K2_GetComponentLocation` _capsulecomponent) (* (`KismetMathLibrary.GetForwardVector` (`SceneComponent.K2_GetComponentRotation` _capsulecomponent)) 10.0)) :`End` (+ (`SceneComponent.K2_GetComponentLocation` _capsulecomponent) (* (`KismetMathLibrary.GetForwardVector` (`SceneComponent.K2_GetComponentRotation` (`self.FollowCamera`))) 1000.0)) :`TraceChannel` "TraceTypeQuery1" :`DrawDebugType` "ForDuration"))
        (if _returnvalue
          (bind (_bblockinghit _binitialoverlap _time _distance _location _impactpoint _normal _impactnormal _physmat _hitactor _hitcomponent) (`GameplayStatics.BreakHitResult` _outhit))
          (`PhysicsHandleComponent.GrabComponentAtLocationWithRotation` :`self` (`self.PhysicsHandle`) :`Component` _hitcomponent :`Location` (`SceneComponent.K2_GetComponentLocation` _hitcomponent))
          (set `self.GrapObject` true))))))

(fn `UserConstructionScript`
  (`parent.UserConstructionScript`))