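; BP_GoKart is a drivable Chaos wheeled go-kart with throttle/brake, steering, handbrake and a toggle between two cameras.
; Axis and action inputs feed the vehicle movement component and controller look rotation.
; Each tick, the averaged front steer angle of wheels 0 and 1 drives steering values in the kart and driver mannequin AnimBPs.
; The construction script tints the body through a dynamic material and optionally hides the driver.
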(event `self.ReceiveBeginPlay`
  ;[1 1 1] Setup
  (bind _assk_gokart_skeleton_anim_blueprint (cast `/Game/Gokart/Meshes/SK_Gokart_Skeleton_AnimBlueprint` (`SkeletalMeshComponent.GetAnimInstance` (`self.Mesh`))))
  (set `self.AnimInstance` _assk_gokart_skeleton_anim_blueprint)
  (bind _assk_mannequin_anim_blueprint (cast `/Game/Gokart/Demo/Mannequins/Meshes/SK_Mannequin_AnimBlueprint` (`SkeletalMeshComponent.GetAnimInstance` (`self.Mannequin`))))
  (set `self.CharAnimInstance` _assk_mannequin_anim_blueprint)
  (bind _aschaos_wheeled_vehicle_movement_component (cast `ChaosWheeledVehicleMovementComponent` (`self.VehicleMovementComponent`)))
  (set `self.ChaosComp` _aschaos_wheeled_vehicle_movement_component))

(event `self.ReceiveTick`
  (params (DeltaSeconds :type "Float (single-precision)"))
  (bind _animinstance (`self.AnimInstance`))
  (bind _wheels (`ChaosWheeledVehicleMovementComponent.Wheels` (`self.ChaosComp`)))
  (bind _returnvalue (* (/ (+ (`ChaosVehicleWheel.GetSteerAngle` (`|GetArrayItem` _wheels)) (`ChaosVehicleWheel.GetSteerAngle` (`|GetArrayItem` _wheels 1))) 2.0) 0.74))
  ;[1 1 1] Steering Wheel
  (set `/Game/Gokart/Meshes/SK_Gokart_Skeleton_AnimBlueprint.Steering` (`KismetMathLibrary.MakeRotator` _returnvalue) _animinstance)
  (set `/Game/Gokart/Meshes/SK_Gokart_Skeleton_AnimBlueprint.Joint` (`KismetMathLibrary.MakeVector` 0.0 (/ _returnvalue -7.0)) _animinstance)
  (set `/Game/Gokart/Demo/Mannequins/Meshes/SK_Mannequin_AnimBlueprint.Steering` (/ _returnvalue 40.0) (`self.CharAnimInstance`)))

(event `InputAxis|MoveForward` :overrideparent false
  (params (AxisValue :type "Float (single-precision)"))
  (bind _vehiclemovementcomponent (`self.VehicleMovementComponent`))
  ;[1 1 1] Throttle Input
  (`|ExecutionSequence`
    (:`then_0`
      (if (>= AxisValue 0.0)
        (`ChaosVehicleMovementComponent.SetThrottleInput` _vehiclemovementcomponent AxisValue)
        (`ChaosVehicleMovementComponent.SetBrakeInput` _vehiclemovementcomponent 0.0)
        (else
          (`ChaosVehicleMovementComponent.SetBrakeInput` _vehiclemovementcomponent (* AxisValue -1.0))
          (`ChaosVehicleMovementComponent.SetThrottleInput` _vehiclemovementcomponent 0.0))))))

(event `InputAxis|MoveRight` :overrideparent false
  (params (AxisValue :type "Float (single-precision)"))
  ;[1 1 1] Steering input
  (`ChaosVehicleMovementComponent.SetSteeringInput` (`self.VehicleMovementComponent`) AxisValue))

(event `InputAction|Handbrake`
  (params (Key :type "Key Structure"))
  (bind _vehiclemovementcomponent (`self.VehicleMovementComponent`))
  ;[1 1 1] Handbrake input
  (:`Pressed`
    (`ChaosVehicleMovementComponent.SetHandbrakeInput` _vehiclemovementcomponent true))
  (:`Released`
    (`ChaosVehicleMovementComponent.SetHandbrakeInput` _vehiclemovementcomponent false)))

(event `InputAction|ToggleView`
  (params (Key :type "Key Structure"))
  ;[1 1 1] Switching Camera
  (:`Pressed`
    (`/Engine/EditorBlueprintResources/StandardMacros.FlipFlop`
      (:`A`
        (`ActorComponent.SetActive` (`self.CameraFP`) true false)
        (`ActorComponent.SetActive` (`self.Camera`) false false))
      (:`B`
        (`ActorComponent.SetActive` (`self.Camera`) true false)
        (`ActorComponent.SetActive` (`self.CameraFP`) false false)))))

(event `InputAxis|Turn`
  (params (AxisValue :type "Float (single-precision)"))
  ;[1 1 1] Camera Movement
  (`self.AddControllerYawInput` AxisValue))

(event `InputAxis|LookUp`
  (params (AxisValue :type "Float (single-precision)"))
  ;[1 1 1] Camera Movement
  (`self.AddControllerPitchInput` AxisValue))

(fn `UserConstructionScript`
  (`|ExecutionSequence`
    (:`then_0`
      (`/Engine/EditorBlueprintResources/StandardMacros.IsValid` (`self.BodyMat`)
        (:`Is Not Valid`
          (bind _returnvalue (`PrimitiveComponent.CreateDynamicMaterialInstance` (`self.Mesh`) 0 null "None"))
          (set `self.BodyMat` _returnvalue))))
    (:`then_1`
      (`MaterialInstanceDynamic.SetVectorParameterValue` (`self.BodyMat`) "Base Color" (`self.Color`)))
    (:`then_2`
      (if (not (`self.ShowDriver`))
        (`SceneComponent.SetVisibility` (`self.Mannequin`) false false)))))