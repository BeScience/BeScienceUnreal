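; Modular first-floor facade piece for a Venice-style building, assembled in the construction script from editable options.
; It builds a flat wall, window, doorway or storefront, applying a selected wall material or brick to the M_wall slot.
; Doors and some storefront extras snap to the base mesh's first socket; storefronts can add an awning or sign.
; Flat wall, window and doorway variants can also get left and right corner quoins.
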(fn `UserConstructionScript`
  (bind _wall_or_brick_mat (`self.Wall_or_Brick_MAT`))
  (bind _returnvalue (`KismetMathLibrary.Conv_ByteToInt` (`self.storefront`)))
  (bind _output (`|GetArrayItem` (`self.Wall_MATs`) (`KismetMathLibrary.Conv_ByteToInt` (`self.Wall_MAT`))))
  (if (`self.flat_wall`)
    (bind _returnvalue_2 (`AddComponent|NODE_AddStaticMeshComponent-7`))
    (if (`self.Wall_or_Brick_MAT`)
      (`PrimitiveComponent.SetMaterialByName` _returnvalue_2 "M_wall" (`|GetArrayItem` (`self.Wall_MATs`) (`KismetMathLibrary.Conv_ByteToInt` (`self.Wall_MAT`))))
      (else
        (`PrimitiveComponent.SetMaterialByName` _returnvalue_2 "M_wall" "/Game/Environments/Venice_fast_building/Materials/MI_brick_wall_01.MI_brick_wall_01")))
    (`self.quoin`)
    (else
      (switch `/Game/Environments/Venice_fast_building/Blueprints/lists_structs/E_window_doorway_storefront` (`self.window_doorway_storefront`)
        (:`NewEnumerator0`
          (if (`self.W_single_double`)
            (bind _returnvalue_3 (`AddComponent|NODE_AddStaticMeshComponent-8`))
            (if _wall_or_brick_mat
              (`PrimitiveComponent.SetMaterialByName` _returnvalue_3 "M_wall" _output)
              (else
                (`PrimitiveComponent.SetMaterialByName` _returnvalue_3 "M_wall" "/Game/Environments/Venice_fast_building/Materials/MI_brick_wall_01.MI_brick_wall_01" :!label _label)
                (`PrimitiveComponent.SetMaterialByName` (stale _returnvalue_4) "M_wall" "/Game/Environments/Venice_fast_building/Materials/MI_brick_wall_01.MI_brick_wall_01")))
            (else
              (bind _returnvalue_4 (`AddComponent|NODE_AddStaticMeshComponent-9`))
              (if _wall_or_brick_mat
                (`PrimitiveComponent.SetMaterialByName` _returnvalue_4 "M_wall" _output)
                (else
                  (goto _label)))))
          (`self.quoin`))
        (:`NewEnumerator1`
          (bind _returnvalue_5 (`AddComponent|NODE_AddStaticMeshComponent-0`))
          (bind _output_get (set `self.current_mesh` _returnvalue_5))
          (`StaticMeshComponent.SetStaticMesh` _output_get (`|GetArrayItem` (`self.Doorways`) (`KismetMathLibrary.Conv_ByteToInt` (`self.doorway`))))
          (if (`self.Wall_or_Brick_MAT`)
            (`PrimitiveComponent.SetMaterialByName` _output_get "M_wall" (`|GetArrayItem` (`self.Wall_MATs`) (`KismetMathLibrary.Conv_ByteToInt` (`self.Wall_MAT`))))
            (else
              (`PrimitiveComponent.SetMaterialByName` _output_get "M_wall" "/Game/Environments/Venice_fast_building/Materials/MI_brick_wall_01.MI_brick_wall_01")))
          (bind _returnvalue_6 (`AddComponent|NODE_AddStaticMeshComponent-3` :`RelativeTransform` (`SceneComponent.GetSocketTransform` _output_get (`|GetArrayItem` (`SceneComponent.GetAllSocketNames` _output_get)) "RTS_Component")))
          (`StaticMeshComponent.SetStaticMesh` _returnvalue_6 (`|GetArrayItem` (`self.doors`) (`KismetMathLibrary.Conv_ByteToInt` (`self.door`))))
          (`PrimitiveComponent.SetMaterial` _returnvalue_6 0 (`|GetArrayItem` (`self.Wood_MATs`) (`KismetMathLibrary.Conv_ByteToInt` (`self.Door_MAT`))))
          (`self.quoin`))
        (:`NewEnumerator2`
          (bind _returnvalue_7 (`AddComponent|NODE_AddStaticMeshComponent-1`))
          (bind _output_get_2 (set `self.current_mesh` _returnvalue_7))
          (`StaticMeshComponent.SetStaticMesh` _output_get_2 (`|GetArrayItem` (`self.Storefronts`) _returnvalue))
          (if (`self.Wall_or_Brick_MAT`)
            (`PrimitiveComponent.SetMaterialByName` _output_get_2 "M_wall" (`|GetArrayItem` (`self.Wall_MATs`) (`KismetMathLibrary.Conv_ByteToInt` (`self.Wall_MAT`))))
            (else
              (`PrimitiveComponent.SetMaterialByName` _output_get_2 "M_wall" "/Game/Environments/Venice_fast_building/Materials/MI_brick_wall_01.MI_brick_wall_01")))
          (if (`KismetMathLibrary.Conv_IntToBool` (`KismetArrayLibrary.Array_Length` (`SceneComponent.GetAllSocketNames` _output_get_2)))
            (`AddComponent|NODE_AddStaticMeshComponent-2` :`RelativeTransform` (`SceneComponent.GetSocketTransform` _output_get_2 (`|GetArrayItem` (`SceneComponent.GetAllSocketNames` _output_get_2)) "RTS_Component")))
          (switch `/Game/Environments/Venice_fast_building/Blueprints/lists_structs/E_awning_sign_nothing` (`self.awning_sign_nothing`)
            (:`NewEnumerator0`
              (bind _returnvalue_8 (`AddComponent|NODE_AddStaticMeshComponent-6`))
              (`PrimitiveComponent.SetMaterial` _returnvalue_8 1 (`|GetArrayItem` (`self.Awning_MATs`) (`KismetMathLibrary.Conv_ByteToInt` (`self.Awning_MAT`)))))
            (:`NewEnumerator1`
              (switch `int` _returnvalue
                (:`0`
                  (`AddComponent|NODE_AddStaticMeshComponent-4` :!label _label_2))
                (:`1`
                  (goto _label_2))
                (:`2`
                  (`AddComponent|NODE_AddStaticMeshComponent-5` :!label _label_3))
                (:`3`
                  (goto _label_3))
                (:`4`
                  (goto _label_3))
                (:`5`
                  (goto _label_3))))))))))