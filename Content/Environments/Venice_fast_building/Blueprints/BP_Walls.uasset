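; Modular Venice building wall piece that assembles itself from static mesh components in its construction script, based on editable options.
; It builds a flat, window or window-balcony wall for the chosen type, with optional quoins, downspouts, sills, railings, awnings and balconies.
; Window and balcony parts attach at the wall mesh's first socket, and wall materials switch between a selectable set and brick.
; A seeded random stream picks leak decal meshes.
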(fn `UserConstructionScript`
  (bind _returnvalue (`KismetMathLibrary.MakeTransform` (0.0 -300.0 0.0) (struct :`Yaw` -90.0)))
  (bind _output (`|GetArrayItem` (`self.Wall MATs`) (`KismetMathLibrary.Conv_ByteToInt` (`self.wall MAT`))))
  (bind _returnvalue_2 (select `/Game/Environments/Venice_fast_building/Blueprints/lists_structs/E_WorWB` (`self.W_or_WB`) :`NewEnumerator0` _returnvalue :`NewEnumerator1` (select `/Game/Environments/Venice_fast_building/Blueprints/lists_structs/E_single_double_triple` (`self.WB_single_double_triple`) :`NewEnumerator0` _returnvalue :`NewEnumerator1` _returnvalue :`NewEnumerator2` (`KismetMathLibrary.MakeTransform` (0.0 -600.0 0.0) (struct :`Yaw` -90.0)))))
  (`/Engine/EditorBlueprintResources/StandardMacros.CompareInt` (`KismetMathLibrary.BreakRandomStream` (`self.Seed`))
    (:`>`
      _)
    (:`==`
      (`KismetMathLibrary.SeedRandomStream` (`self.Seed`)))
    (:`<`
      _))
  (if (`self.flat_wall`)
    (switch `/Game/Environments/Venice_fast_building/Blueprints/lists_structs/E_window_type_list` (`self.type`)
      (:`NewEnumerator0`
        (bind _returnvalue_3 (`AddComponent|NODE_AddStaticMeshComponent-55`))
        (if (`self.Wall_or_Brick_MAT`)
          (`PrimitiveComponent.SetMaterialByName` _returnvalue_3 "M_wall" _output)
          (else
            (`PrimitiveComponent.SetMaterialByName` _returnvalue_3 "M_wall" "/Game/Environments/Venice_fast_building/Materials/MI_brick_wall_01.MI_brick_wall_01")))
        (if (`self.downspout`)
          (if (`self.downspout end`)
            (`AddComponent|NODE_AddStaticMeshComponent-58`)
            (else
              (`AddComponent|NODE_AddStaticMeshComponent-56`)))))
      (:`NewEnumerator1`
        (bind _returnvalue_4 (`AddComponent|NODE_AddStaticMeshComponent-54` :!label _label))
        (if (`self.Wall_or_Brick_MAT`)
          (`PrimitiveComponent.SetMaterialByName` _returnvalue_4 "M_wall" _output)
          (else
            (`PrimitiveComponent.SetMaterialByName` _returnvalue_4 "M_wall" "/Game/Environments/Venice_fast_building/Materials/MI_brick_wall_01.MI_brick_wall_01")))
        (if (`self.downspout`)
          (if (`self.downspout end`)
            (`AddComponent|NODE_AddStaticMeshComponent-59`)
            (else
              (`AddComponent|NODE_AddStaticMeshComponent-57`)))))
      (:`NewEnumerator2`
        (goto _label))
      (:`NewEnumerator3`
        (goto _label))
      (:`NewEnumerator4`
        (goto _label)))
    (else
      (switch `/Game/Environments/Venice_fast_building/Blueprints/lists_structs/E_WorWB` (`self.W_or_WB`)
        (:`NewEnumerator0`
          (`self.windows`))
        (:`NewEnumerator1`
          (`self.windows_baclony`)))))
  (if (`self.quoin_on_left`)
    (switch `/Game/Environments/Venice_fast_building/Blueprints/lists_structs/E_window_type_list` (`self.type`)
      (:`NewEnumerator0`
        (`AddComponent|NODE_AddStaticMeshComponent-60`))
      (:`NewEnumerator1`
        (`AddComponent|NODE_AddStaticMeshComponent-61` :!label _label_2))
      (:`NewEnumerator2`
        (goto _label_2))
      (:`NewEnumerator3`
        (goto _label_2))
      (:`NewEnumerator4`
        (goto _label_2))))
  (if (`self.quoin_on_right`)
    (switch `/Game/Environments/Venice_fast_building/Blueprints/lists_structs/E_window_type_list` (`self.type`)
      (:`NewEnumerator0`
        (`AddComponent|NODE_AddStaticMeshComponent-62` :`RelativeTransform` _returnvalue_2))
      (:`NewEnumerator1`
        (`AddComponent|NODE_AddStaticMeshComponent-63` :`RelativeTransform` _returnvalue_2 :!label _label_3))
      (:`NewEnumerator2`
        (goto _label_3))
      (:`NewEnumerator3`
        (goto _label_3))
      (:`NewEnumerator4`
        (goto _label_3)))))

(fn `windows`
  (bind (_center _left _right _double) (`self.W Walls selector` (`self.type`)))
  (bind (_001 _002 _003 _004) (`self.W Windows selector` (`self.type`)))
  (bind _output (`|GetArrayItem` (`self.Wall MATs`) (`KismetMathLibrary.Conv_ByteToInt` (`self.wall MAT`))))
  (bind _output_2 (`|GetArrayItem` (`self.Wall MATs`) (`KismetMathLibrary.Conv_ByteToInt` (`self.wall MAT`))))
  (switch `/Game/Environments/Venice_fast_building/Blueprints/lists_structs/E_window_placement_list` (`self.W_placement`)
    (:`NewEnumerator1`
      (bind _returnvalue (`AddComponent|NODE_AddStaticMeshComponent-8` :`RelativeTransform` (`self.transform`)))
      (bind _output_get (set `self.current mesh` _returnvalue))
      (`StaticMeshComponent.SetStaticMesh` _output_get _center)
      (if (`self.Wall_or_Brick_MAT`)
        (`PrimitiveComponent.SetMaterialByName` _returnvalue "M_wall" _output_2)
        (else
          (`PrimitiveComponent.SetMaterialByName` _returnvalue "M_wall" "/Game/Environments/Venice_fast_building/Materials/MI_brick_wall_01.MI_brick_wall_01")))
      (set `self.socket RP` (`self.Get SOCKET RP`))
      (if (`self.Open`) :!label _label
        (bind _returnvalue_2 (`AddComponent|NODE_AddStaticMeshComponent-12` :`RelativeTransform` (`self.socket RP`)))
        (bind _output_get_2 (set `self.current mesh` _returnvalue_2))
        (`StaticMeshComponent.SetStaticMesh` _output_get_2 _001)
        (else
          (bind _returnvalue_3 (`AddComponent|NODE_AddStaticMeshComponent-13` :`RelativeTransform` (`self.socket RP`)))
          (bind _output_get_3 (set `self.current mesh` _returnvalue_3))
          (`StaticMeshComponent.SetStaticMesh` _output_get_3 _002)))
      (if (`self.Wall_or_Brick_MAT`)
        (`PrimitiveComponent.SetMaterialByName` _returnvalue_3 "M_wall" _output)
        (`PrimitiveComponent.SetMaterialByName` _returnvalue_2 "M_wall" _output)
        (else
          (`PrimitiveComponent.SetMaterialByName` _returnvalue_3 "M_wall" "/Game/Environments/Venice_fast_building/Materials/MI_brick_wall_01.MI_brick_wall_01")
          (`PrimitiveComponent.SetMaterialByName` _returnvalue_2 "M_wall" "/Game/Environments/Venice_fast_building/Materials/MI_brick_wall_01.MI_brick_wall_01")))
      (if (`self.W_sill`)
        (`AddComponent|NODE_AddStaticMeshComponent-16` :`RelativeTransform` (`self.socket RP`))
        (if (`self.W_railing`)
          (`AddComponent|NODE_AddStaticMeshComponent-17` :`RelativeTransform` (`self.socket RP`))))
      (if (and (`self.W_awning`) (`self.Open`))
        (bind _returnvalue_4 (`AddComponent|NODE_AddStaticMeshComponent-38` :`RelativeTransform` (`self.socket RP`)))
        (`PrimitiveComponent.SetMaterial` _returnvalue_4 1 (`|GetArrayItem` (`self.Awning MATs`) (`KismetMathLibrary.Conv_ByteToInt` (`self.W_awning color`)))))
      (if (`self.W_leaks`)
        (bind _returnvalue_5 (`AddComponent|NODE_AddStaticMeshComponent-39` :`RelativeTransform` (`self.socket RP`)))
        (`StaticMeshComponent.SetStaticMesh` _returnvalue_5 (`|GetArrayItem` (`self.Leaks_single`) (`KismetMathLibrary.RandomIntegerInRangeFromStream` (`self.Seed`) 0 4))))
      (if (`self.downspout`) :!label _label_2
        (switch `/Game/Environments/Venice_fast_building/Blueprints/lists_structs/E_window_type_list` (`self.type`)
          (:`NewEnumerator0`
            (if (`self.downspout end`)
              (`AddComponent|NODE_AddStaticMeshComponent-43`)
              (else
                (`AddComponent|NODE_AddStaticMeshComponent-41`))))
          (:`NewEnumerator1`
            (if (`self.downspout end`) :!label _label_3
              (`AddComponent|NODE_AddStaticMeshComponent-44`)
              (else
                (`AddComponent|NODE_AddStaticMeshComponent-42`))))
          (:`NewEnumerator2`
            (goto _label_3))
          (:`NewEnumerator3`
            (goto _label_3))
          (:`NewEnumerator4`
            (goto _label_3)))))
    (:`NewEnumerator2`
      (bind _returnvalue_6 (`AddComponent|NODE_AddStaticMeshComponent-9` :`RelativeTransform` (`self.transform`)))
      (bind _output_get_4 (set `self.current mesh` _returnvalue_6))
      (`StaticMeshComponent.SetStaticMesh` _output_get_4 _left)
      (if (`self.Wall_or_Brick_MAT`)
        (`PrimitiveComponent.SetMaterialByName` _returnvalue_6 "M_wall" _output_2)
        (else
          (`PrimitiveComponent.SetMaterialByName` _returnvalue_6 "M_wall" "/Game/Environments/Venice_fast_building/Materials/MI_brick_wall_01.MI_brick_wall_01")))
      (set `self.socket RP` (`self.Get SOCKET RP`))
      (goto _label))
    (:`NewEnumerator0`
      (bind _returnvalue_7 (`AddComponent|NODE_AddStaticMeshComponent-10` :`RelativeTransform` (`self.transform`)))
      (bind _output_get_5 (set `self.current mesh` _returnvalue_7))
      (`StaticMeshComponent.SetStaticMesh` _output_get_5 _right)
      (if (`self.Wall_or_Brick_MAT`)
        (`PrimitiveComponent.SetMaterialByName` _returnvalue_7 "M_wall" _output_2)
        (else
          (`PrimitiveComponent.SetMaterialByName` _returnvalue_7 "M_wall" "/Game/Environments/Venice_fast_building/Materials/MI_brick_wall_01.MI_brick_wall_01")))
      (set `self.socket RP` (`self.Get SOCKET RP`))
      (goto _label))
    (:`NewEnumerator3`
      (bind _returnvalue_8 (`AddComponent|NODE_AddStaticMeshComponent-11` :`RelativeTransform` (`self.transform`)))
      (bind _output_get_6 (set `self.current mesh` _returnvalue_8))
      (`StaticMeshComponent.SetStaticMesh` _output_get_6 _double)
      (if (`self.Wall_or_Brick_MAT`)
        (`PrimitiveComponent.SetMaterialByName` _returnvalue_8 "M_wall" _output_2)
        (else
          (`PrimitiveComponent.SetMaterialByName` _returnvalue_8 "M_wall" "/Game/Environments/Venice_fast_building/Materials/MI_brick_wall_01.MI_brick_wall_01")))
      (set `self.socket RP` (`self.Get SOCKET RP`))
      (if (`self.Open`)
        (bind _returnvalue_9 (`AddComponent|NODE_AddStaticMeshComponent-14` :`RelativeTransform` (`self.socket RP`)))
        (bind _output_get_7 (set `self.current mesh` _returnvalue_9))
        (`StaticMeshComponent.SetStaticMesh` _output_get_7 _003)
        (else
          (bind _returnvalue_10 (`AddComponent|NODE_AddStaticMeshComponent-15` :`RelativeTransform` (`self.socket RP`)))
          (bind _output_get_8 (set `self.current mesh` _returnvalue_10))
          (`StaticMeshComponent.SetStaticMesh` _output_get_8 _004)))
      (if (`self.Wall_or_Brick_MAT`)
        (`PrimitiveComponent.SetMaterialByName` _returnvalue_10 "M_wall" _output)
        (`PrimitiveComponent.SetMaterialByName` _returnvalue_9 "M_wall" _output)
        (else
          (`PrimitiveComponent.SetMaterialByName` _returnvalue_10 "M_wall" "/Game/Environments/Venice_fast_building/Materials/MI_brick_wall_01.MI_brick_wall_01")
          (`PrimitiveComponent.SetMaterialByName` _returnvalue_9 "M_wall" "/Game/Environments/Venice_fast_building/Materials/MI_brick_wall_01.MI_brick_wall_01")))
      (if (`self.W_leaks`)
        (bind _returnvalue_11 (`AddComponent|NODE_AddStaticMeshComponent-40` :`RelativeTransform` (`self.socket RP`)))
        (`StaticMeshComponent.SetStaticMesh` _returnvalue_11 (`|GetArrayItem` (`self.Leaks_double`) (`KismetMathLibrary.RandomIntegerInRangeFromStream` (`self.Seed`) 0 3)))
        (else
          (goto _label_2))))))

(fn `windows_baclony`
  (bind _wb_balconys_list (`self.WB_balconys_list`))
  (bind (_single _double _triple) (`self.WB Walls selector` (`self.type`)))
  (bind (_001 _002 _003 _004 _005 _006) (`self.WB Windows selector` (`self.type`)))
  (bind _output (`|GetArrayItem` (`self.Wall MATs`) (`KismetMathLibrary.Conv_ByteToInt` (`self.wall MAT`))))
  (switch `/Game/Environments/Venice_fast_building/Blueprints/lists_structs/E_single_double_triple` (`self.WB_single_double_triple`)
    (:`NewEnumerator0`
      (bind _returnvalue (`AddComponent|NODE_AddStaticMeshComponent-19` :`RelativeTransform` (`self.transform`)))
      (bind _output_get (set `self.current mesh` _returnvalue))
      (`StaticMeshComponent.SetStaticMesh` _output_get _single)
      (if (`self.Wall_or_Brick_MAT`)
        (`PrimitiveComponent.SetMaterialByName` _returnvalue "M_wall" _output)
        (else
          (`PrimitiveComponent.SetMaterialByName` _returnvalue "M_wall" "/Game/Environments/Venice_fast_building/Materials/MI_brick_wall_01.MI_brick_wall_01")))
      (set `self.socket RP` (`self.Get SOCKET RP`))
      (if (`self.Open`)
        (if (`self.WB_balustrade`)
          (bind _returnvalue_2 (`AddComponent|NODE_AddStaticMeshComponent-24` :`RelativeTransform` (`self.socket RP`)))
          (bind _output_get_2 (set `self.current mesh` _returnvalue_2))
          (`StaticMeshComponent.SetStaticMesh` _output_get_2 _003)
          (if (`self.Wall_or_Brick_MAT`)
            (`PrimitiveComponent.SetMaterialByName` _returnvalue_2 "M_wall" null)
            (else
              (`PrimitiveComponent.SetMaterialByName` _returnvalue_2 "M_wall" "/Game/Environments/Venice_fast_building/Materials/MI_brick_wall_01.MI_brick_wall_01")))
          (switch `/Game/Environments/Venice_fast_building/Blueprints/lists_structs/E_balconys_list` _wb_balconys_list :!label _label
            (:`NewEnumerator0`
              (`AddComponent|NODE_AddStaticMeshComponent-28` :`RelativeTransform` (`self.socket RP`) :!label _label_2))
            (:`NewEnumerator1`
              (goto _label_2))
            (:`NewEnumerator2`
              (goto _label_2))
            (:`NewEnumerator3`
              _))
          (else
            (bind _returnvalue_3 (`AddComponent|NODE_AddStaticMeshComponent-22` :`RelativeTransform` (`self.socket RP`)))
            (bind _output_get_3 (set `self.current mesh` _returnvalue_3))
            (`StaticMeshComponent.SetStaticMesh` _output_get_3 _001)
            (if (`self.Wall_or_Brick_MAT`)
              (`PrimitiveComponent.SetMaterialByName` _returnvalue_3 "M_wall" (`|GetArrayItem` (`self.Wall MATs`) (`KismetMathLibrary.Conv_ByteToInt` (`self.wall MAT`))))
              (else
                (`PrimitiveComponent.SetMaterialByName` _returnvalue_3 "M_wall" "/Game/Environments/Venice_fast_building/Materials/MI_brick_wall_01.MI_brick_wall_01")))
            (switch `/Game/Environments/Venice_fast_building/Blueprints/lists_structs/E_balconys_list` (`self.WB_balconys_list`) :!label _label_3
              (:`NewEnumerator0`
                (`AddComponent|NODE_AddStaticMeshComponent-29` :`RelativeTransform` (`self.socket RP`)))
              (:`NewEnumerator1`
                (`AddComponent|NODE_AddStaticMeshComponent-31` :`RelativeTransform` (`self.socket RP`)))
              (:`NewEnumerator2`
                (`AddComponent|NODE_AddStaticMeshComponent-33` :`RelativeTransform` (`self.socket RP`)))
              (:`NewEnumerator3`
                _))))
        (else
          (bind _returnvalue_4 (`AddComponent|NODE_AddStaticMeshComponent-23` :`RelativeTransform` (`self.socket RP`)))
          (bind _output_get_4 (set `self.current mesh` _returnvalue_4))
          (`StaticMeshComponent.SetStaticMesh` _output_get_4 _002)
          (if (`self.Wall_or_Brick_MAT`)
            (`PrimitiveComponent.SetMaterialByName` _returnvalue_4 "M_wall" null)
            (else
              (`PrimitiveComponent.SetMaterialByName` _returnvalue_4 "M_wall" "/Game/Environments/Venice_fast_building/Materials/MI_brick_wall_01.MI_brick_wall_01")))
          (if (`self.WB_balustrade`)
            (goto _label)
            (else
              (goto _label_3))))))
    (:`NewEnumerator1`
      (bind _returnvalue_5 (`AddComponent|NODE_AddStaticMeshComponent-20` :`RelativeTransform` (`self.transform`)))
      (bind _output_get_5 (set `self.current mesh` _returnvalue_5))
      (`StaticMeshComponent.SetStaticMesh` _output_get_5 _double)
      (if (`self.Wall_or_Brick_MAT`)
        (`PrimitiveComponent.SetMaterialByName` _returnvalue_5 "M_wall" _output)
        (else
          (`PrimitiveComponent.SetMaterialByName` _returnvalue_5 "M_wall" "/Game/Environments/Venice_fast_building/Materials/MI_brick_wall_01.MI_brick_wall_01")))
      (set `self.socket RP` (`self.Get SOCKET RP`))
      (if (`self.Open`)
        (bind _returnvalue_6 (`AddComponent|NODE_AddStaticMeshComponent-25` :`RelativeTransform` (`self.socket RP`)))
        (bind _output_get_6 (set `self.current mesh` _returnvalue_6))
        (`StaticMeshComponent.SetStaticMesh` _output_get_6 _004)
        (if (`self.Wall_or_Brick_MAT`)
          (`PrimitiveComponent.SetMaterialByName` _returnvalue_6 "M_wall" null)
          (else
            (`PrimitiveComponent.SetMaterialByName` _returnvalue_6 "M_wall" "/Game/Environments/Venice_fast_building/Materials/MI_brick_wall_01.MI_brick_wall_01")))
        (else
          (bind _returnvalue_7 (`AddComponent|NODE_AddStaticMeshComponent-26` :`RelativeTransform` (`self.socket RP`)))
          (bind _output_get_7 (set `self.current mesh` _returnvalue_7))
          (`StaticMeshComponent.SetStaticMesh` _output_get_7 _005)
          (if (`self.Wall_or_Brick_MAT`)
            (`PrimitiveComponent.SetMaterialByName` _returnvalue_7 "M_wall" null)
            (else
              (`PrimitiveComponent.SetMaterialByName` _returnvalue_7 "M_wall" "/Game/Environments/Venice_fast_building/Materials/MI_brick_wall_01.MI_brick_wall_01")))))
      (switch `/Game/Environments/Venice_fast_building/Blueprints/lists_structs/E_balconys_list` _wb_balconys_list
        (:`NewEnumerator0`
          (`AddComponent|NODE_AddStaticMeshComponent-30` :`RelativeTransform` (`self.socket RP`)))
        (:`NewEnumerator1`
          (`AddComponent|NODE_AddStaticMeshComponent-32` :`RelativeTransform` (`self.socket RP`)))
        (:`NewEnumerator2`
          (`AddComponent|NODE_AddStaticMeshComponent-34` :`RelativeTransform` (`self.socket RP`)))
        (:`NewEnumerator3`
          _)))
    (:`NewEnumerator2`
      (bind _returnvalue_8 (`AddComponent|NODE_AddStaticMeshComponent-21` :`RelativeTransform` (`self.transform`)))
      (bind _output_get_8 (set `self.current mesh` _returnvalue_8))
      (`StaticMeshComponent.SetStaticMesh` _output_get_8 _triple)
      (if (`self.Wall_or_Brick_MAT`)
        (`PrimitiveComponent.SetMaterialByName` _returnvalue_8 "M_wall" _output)
        (else
          (`PrimitiveComponent.SetMaterialByName` _returnvalue_8 "M_wall" "/Game/Environments/Venice_fast_building/Materials/MI_brick_wall_01.MI_brick_wall_01")))
      (set `self.socket RP` (`self.Get SOCKET RP`))
      (bind _returnvalue_9 (`AddComponent|NODE_AddStaticMeshComponent-27` :`RelativeTransform` (`self.socket RP`)))
      (bind _output_get_9 (set `self.current mesh` _returnvalue_9))
      (`StaticMeshComponent.SetStaticMesh` _output_get_9 _006)
      (if (`self.Wall_or_Brick_MAT`)
        (`PrimitiveComponent.SetMaterialByName` _returnvalue_9 "M_wall" null)
        (else
          (`PrimitiveComponent.SetMaterialByName` _returnvalue_9 "M_wall" "/Game/Environments/Venice_fast_building/Materials/MI_brick_wall_01.MI_brick_wall_01")))
      (switch `/Game/Environments/Venice_fast_building/Blueprints/lists_structs/E_balconys_list` (`self.WB_balconys_list`)
        (:`NewEnumerator0`
          (`AddComponent|NODE_AddStaticMeshComponent-35` :`RelativeTransform` (`self.socket RP`)))
        (:`NewEnumerator1`
          (`AddComponent|NODE_AddStaticMeshComponent-36` :`RelativeTransform` (`self.socket RP`)))
        (:`NewEnumerator2`
          (`AddComponent|NODE_AddStaticMeshComponent-37` :`RelativeTransform` (`self.socket RP`)))
        (:`NewEnumerator3`
          _))))
  (if (`self.downspout`)
    (switch `/Game/Environments/Venice_fast_building/Blueprints/lists_structs/E_window_type_list` (`self.type`)
      (:`NewEnumerator0`
        (if (`self.downspout end`)
          (`AddComponent|NODE_AddStaticMeshComponent-51`)
          (else
            (`AddComponent|NODE_AddStaticMeshComponent-49`))))
      (:`NewEnumerator1`
        (if (`self.downspout end`) :!label _label_4
          (`AddComponent|NODE_AddStaticMeshComponent-52`)
          (else
            (`AddComponent|NODE_AddStaticMeshComponent-50`))))
      (:`NewEnumerator2`
        (goto _label_4))
      (:`NewEnumerator3`
        (goto _label_4))
      (:`NewEnumerator4`
        (goto _label_4)))))