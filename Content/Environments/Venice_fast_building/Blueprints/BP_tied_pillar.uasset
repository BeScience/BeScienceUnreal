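; BP_tied_pillar is a pillar prop Blueprint from the Venice fast building environment set.
; Its Construction Script adds one of two static mesh components based on WoodenOrMetallic.
; When the flag is true, it creates a dynamic instance of M_stripes on the mesh and feeds in both stripe colors and an inverted MoldHeight as the mold Z shift.
; The event graph has no active logic.
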(fn `UserConstructionScript`
  (if (`self.Wooden_or_metallic`)
    (bind _returnvalue (`AddComponent|NODE_AddStaticMeshComponent-0`))
    (bind _returnvalue_2 (`PrimitiveComponent.CreateDynamicMaterialInstance` _returnvalue 0 "/Game/Environments/Venice_fast_building/Materials/M_stripes.M_stripes" "None"))
    (`MaterialInstanceDynamic.SetScalarParameterValue` _returnvalue_2 "Mold Z shift" (- 1.0 (`self.Mold height`)))
    (`MaterialInstanceDynamic.SetVectorParameterValue` _returnvalue_2 "color" (`self.color_1`))
    (`MaterialInstanceDynamic.SetVectorParameterValue` _returnvalue_2 "color_2" (`self.color_2`))
    (else
      (`AddComponent|NODE_AddStaticMeshComponent-1`))))