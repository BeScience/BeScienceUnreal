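; Drivable Chaos go-kart pawn with a tinted body and a mannequin driver shown while possessed.
; Axis and action inputs feed throttle, brake, steering and handbrake.
; Tick converts front wheel steer angles into kart and driver animation.
; An optional spawned BP_Opencv actor supplies hand positions and wheel angle, moving visible hand and wheel components, switching hand materials on grip state and feeding CvSteering as an alternative steering source.
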(event `self.ReceiveBeginPlay`
  ;[1 1 1] Setup
  (bind _assk_gokart_skeleton_anim_blueprint (cast `/Game/Swkim/Gokart/Meshes/SK_Gokart_Skeleton_AnimBlueprint` (`SkeletalMeshComponent.GetAnimInstance` (`self.Mesh`))))
  (set `self.AnimInstance` _assk_gokart_skeleton_anim_blueprint)
  (bind _asabp_steel (cast `/Game/Steel/ABP_Steel` (`SkeletalMeshComponent.GetAnimInstance` (`self.Mannequin`))))
  (set `self.CharAnimInstance` _asabp_steel)
  (bind _aschaos_wheeled_vehicle_movement_component (cast `ChaosWheeledVehicleMovementComponent` (`self.VehicleMovementComponent`)))
  (set `self.ChaosComp` _aschaos_wheeled_vehicle_movement_component))

(event `InputAxis|MoveForward` :overrideparent false
  (params (AxisValue :type "Float (single-precision)"))
  (bind _vehiclemovementcomponent (`self.VehicleMovementComponent`))
  ;[1 1 1] Throttle Input
  (`|ExecutionSequence`
    (:`then_0`
      (if (>= AxisValue 0.0)
        (`ChaosVehicleMovementComponent.SetThrottleInput` _vehiclemovementcomponent AxisValue)
        (`ChaosVehicleMovementComponent.SetBrakeInput` _vehiclemovementcomponent 0.0)
        (else
          (`ChaosVehicleMovementComponent.SetBrakeInput` _vehiclemovementcomponent (* AxisValue -1.0))
          (`ChaosVehicleMovementComponent.SetThrottleInput` _vehiclemovementcomponent 0.0))))))

(event `InputAxis|MoveRight` :overrideparent false
  (params (AxisValue :type "Float (single-precision)"))
  ;[1 1 1] Steering input
  (`ChaosVehicleMovementComponent.SetSteeringInput` (`self.VehicleMovementComponent`) AxisValue))

(event `InputAction|Handbrake`
  (params (Key :type "Key Structure"))
  (bind _vehiclemovementcomponent (`self.VehicleMovementComponent`))
  ;[1 1 1] Handbrake input
  (:`Pressed`
    (`ChaosVehicleMovementComponent.SetHandbrakeInput` _vehiclemovementcomponent true))
  (:`Released`
    (`ChaosVehicleMovementComponent.SetHandbrakeInput` _vehiclemovementcomponent false)))

(event `self.ReceiveTick`
  (params (DeltaSeconds :type "Float (single-precision)"))
  (bind _animinstance (`self.AnimInstance`))
  (bind _handleft (`self.HandLeft`))
  (bind _opencv (`self.opencv`))
  (bind _hendright (`self.HendRight`))
  (bind _wheelangle (`BSU_TrackingHand.wheelAngle` (`self.opencv`)))
  (bind _wheels (`ChaosWheeledVehicleMovementComponent.Wheels` (`self.ChaosComp`)))
  (bind _returnvalue (`KismetMathLibrary.MakeRotator` 0.0 _wheelangle 90.0))
  (bind _returnvalue_2 (* (/ (+ (`ChaosVehicleWheel.GetSteerAngle` (`|GetArrayItem` _wheels)) (`ChaosVehicleWheel.GetSteerAngle` (`|GetArrayItem` _wheels 1))) 2.0) 0.74))
  (`|ExecutionSequence`
    (:`then_0`
      ;[1 1 1] Steering Wheel
      (set `/Game/Swkim/Gokart/Meshes/SK_Gokart_Skeleton_AnimBlueprint.Steering` (`KismetMathLibrary.MakeRotator` _returnvalue_2) _animinstance)
      (set `/Game/Swkim/Gokart/Meshes/SK_Gokart_Skeleton_AnimBlueprint.Joint` (`KismetMathLibrary.MakeVector` 0.0 (/ _returnvalue_2 -7.0)) _animinstance)
      (set `/Game/Steel/ABP_Steel.Steeling` (/ _returnvalue_2 40.0) (`self.CharAnimInstance`)))
    (:`then_1`
      (`/Engine/EditorBlueprintResources/StandardMacros.IsValid` _opencv
        (:`Is Valid`
          ;[1 1 1] 손이동처리
          (`|ExecutionSequence`
            (:`then_0`
              (if (`BSU_TrackingHand.is_handle` _opencv)
                (`PrimitiveComponent.SetMaterial` _handleft 0 "/Engine/EngineDebugMaterials/BlackUnlitMaterial.BlackUnlitMaterial")
                (`PrimitiveComponent.SetMaterial` _hendright 0 "/Engine/EngineDebugMaterials/BlackUnlitMaterial.BlackUnlitMaterial")
                (else
                  (`PrimitiveComponent.SetMaterial` _handleft 0 null)
                  (`PrimitiveComponent.SetMaterial` _hendright 0 null))))
            (:`then_1`
              (`SceneComponent.K2_SetRelativeLocationAndRotation` _handleft (`KismetMathLibrary.MakeVector` 45.0 (- (/ (`BSU_TrackingHand.hand_left_x` _opencv) 6.0) 53.0) (- 30.0 (/ (`BSU_TrackingHand.hand_left_y` _opencv) 6.0))) _returnvalue false false)
              (`SceneComponent.K2_SetRelativeLocationAndRotation` _hendright (`KismetMathLibrary.MakeVector` 45.0 (- (/ (`BSU_TrackingHand.hand_right_x` _opencv) 6.0) 53.0) (- 30.0 (/ (`BSU_TrackingHand.hand_right_y` _opencv) 6.0))) _returnvalue false false)
              ;[1 1 1] 카메라 회전로직
              (`SceneComponent.K2_SetRelativeRotation` (`self.SteeringWheel`) _returnvalue false false)
              (`self.CvSteering` (/ (* _wheelangle -1.0) 16.0)))))))))

(event `self.ReceivePossessed`
  (params (NewController :type "Controller Object Reference"))
  (cast `/Game/Kyoulee/BluePrints/GameMode/GamePlay/BP_PC_GamePlay` NewController)
  (`self.MultiShow` true))

(event `self.ReceiveUnpossessed`
  (params (OldController :type "Controller Object Reference"))
  (`self.MultiShow` false))

(event `self.SetupOpencv`
  (`SceneComponent.SetVisibility` (`self.SteeringWheel`) true false)
  (`SceneComponent.SetVisibility` (`self.HendRight`) true false)
  (`SceneComponent.SetVisibility` (`self.HandLeft`) true false)
  (bind _returnvalue (`|SpawnActorFromClass` "/Game/Swkim/Vehicle/BP_Opencv.BP_Opencv_C" (`self.Spawn Transform`) "Undefined" "MultiplyWithRoot" null null))
  (set `self.opencv` _returnvalue))

(event `MultiShow`
  (params (IsShow :type Boolean))
  (`SceneComponent.SetVisibility` (`self.Mannequin`) IsShow false)
  (`KismetSystemLibrary.PrintString` "Hello"))

(event `self.TearDownOpencv`
  (bind _opencv (`self.opencv`))
  (`SceneComponent.SetVisibility` (`self.SteeringWheel`) false false)
  (`SceneComponent.SetVisibility` (`self.HendRight`) false false)
  (`SceneComponent.SetVisibility` (`self.HandLeft`) false false)
  (`/Engine/EditorBlueprintResources/StandardMacros.IsValid` _opencv
    (:`Is Valid`
      (`self.K2_DestroyActor` _opencv))))

(event `self.BrakeLights`
  (params (bBraking :type Boolean)))

(fn `UserConstructionScript`
  (`|ExecutionSequence`
    (:`then_0`
      (`/Engine/EditorBlueprintResources/StandardMacros.IsValid` (`self.BodyMat`)
        (:`Is Not Valid`
          (bind _returnvalue (`PrimitiveComponent.CreateDynamicMaterialInstance` (`self.Mesh`) 0 null "None"))
          (set `self.BodyMat` _returnvalue))))
    (:`then_1`
      (`MaterialInstanceDynamic.SetVectorParameterValue` (`self.BodyMat`) "Base Color" (`self.Color`)))
    (:`then_2`
      (if (not (`self.ShowDriver`))
        (`SceneComponent.SetVisibility` (`self.Mannequin`) false false)))))