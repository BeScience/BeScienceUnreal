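; BP_Opencv is an actor that displays OpenCV frames on screen through the WBP_Opencv widget.
; It creates the widget and adds it to the viewport on BeginPlay, then removes it on EndPlay.
; Tick accumulates time and, once it exceeds SpendTime, calls ReadFrame, resets the timer and pushes ImageTexture into the widget's image brush, throttling the update rate.
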(event `self.ReceiveEndPlay`
  (params (EndPlayReason :type "EEndPlayReason Enum" :default "Destroyed"))
  (`Widget.RemoveFromParent` (`self.OpencvUI`)))

(event `self.ReceiveBeginPlay`
  (bind _returnvalue (`|CreateWidget` "/Game/Swkim/UI/WBP_Opencv.WBP_Opencv_C"))
  (`UserWidget.AddToViewport` _returnvalue 0)
  (set `self.OpencvUI` _returnvalue))

(event `self.ReceiveTick`
  (params (DeltaSeconds :type "Float (single-precision)"))
  (if (> (`self.Current Time`) (`self.Spend Time`))
    (`self.ReadFrame`)
    (set `self.Current Time` 0.0)
    (`Image.SetBrushFromTexture` (`/Game/Swkim/UI/WBP_Opencv.ImageWidget` (`self.OpencvUI`)) (`self.imageTexture`) false)
    (else
      (set `self.Current Time` (+ DeltaSeconds (`self.Current Time`))))))

(fn `UserConstructionScript`)