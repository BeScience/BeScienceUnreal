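; Player character with voice capture for docent NPCs, physics grabbing and camera collision.
; Holding 1 records a WAV that BP_HttpActor sends with the docent's name, but the logic setting Btalk, which gates recording, is disconnected.
; E line-traces for BP_GrabBase objects, relaying PhysicsHandle grab, move and drop through Server and Multicast events.
; Tick updates the held object and sphere-traces to interpolate spring arm length around obstacles.
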(event `self.ReceiveBeginPlay`
  (`|ExecutionSequence`
    (:`then_0`
      (bind _returnvalue (`|SpawnActorFromClass` "/Game/GW/BluePrint/BP_HttpActor.BP_HttpActor_C" (`self.Spawn Transform`) "Undefined" "MultiplyWithRoot" null null))
      (set `self.HttpActor` _returnvalue)
      (set `self.DefaultSpringArmLength` (`SpringArmComponent.TargetArmLength` (`self.SpringArmComp`))))))

(event `Key|One`
  (params (Key :type "Key Structure"))
  (:`Pressed`
    (if (`self.btalk`)
      (`SynthComponent.Start` (`self.AudioCapture`))
      (`AudioMixerBlueprintLibrary.StartRecordingOutput` 0.0 "/Game/GW/Sound/SM_Record.SM_Record")
      (set `self.bVoice` true)
      (`KismetSystemLibrary.PrintString` "Recording" true true (struct :`G` 0.66 :`B` 1.0 :`A` 1.0) 2.0 "-1")))
  (:`Released`
    (if (`self.bVoice`)
      (`SynthComponent.Stop` (`self.AudioCapture`))
      (`AudioMixerBlueprintLibrary.StopRecordingOutput` "WavFile" "test" "" "/Game/GW/Sound/SM_Record.SM_Record" null)
      (`KismetSystemLibrary.PrintString` "RecordingStop" true true (struct :`G` 0.66 :`B` 1.0 :`A` 1.0) 2.0 "1")
      (`KismetSystemLibrary.K2_SetTimerDelegate` (delegate `CustomEvent`) 0.3))))

(event `CustomEvent`
  (`HttpActor.SendSoundWaveFile` (`self.HttpActor`) 0 (`self.DocentName`) (`KismetStringLibrary.Concat_StrStr` (`self.Path`) (`self.Name`))))

(event `self.Sphere.OnComponentBeginOverlap`
  (params (OverlappedComponent :type "PrimitiveComponent Object Reference") (OtherActor :type "Actor Object Reference") (OtherComp :type "PrimitiveComponent Object Reference") (OtherBodyIndex :type Integer) (bFromSweep :type Boolean) (SweepResult :type "HitResult Structure (by ref)")))

(event `Canmeracolision`
  (bind _outhit (`KismetSystemLibrary.SphereTraceSingle` (`SceneComponent.K2_GetComponentLocation` (`self.SpringArmComp`)) (+ (`SceneComponent.K2_GetComponentLocation` (`self.SpringArmComp`)) (* (`KismetMathLibrary.Normal` (- (`SceneComponent.K2_GetComponentLocation` (`self.CameraComp`)) (`SceneComponent.K2_GetComponentLocation` (`self.SpringArmComp`)))) (`self.DefaultSpringArmLength`))) (`self.Radius`) "TraceTypeQuery2" false (`|MakeArray` self :!type "Actor Object Reference") "ForOneFrame"))
  (bind (_bblockinghit _binitialoverlap _time _distance _location _impactpoint) (`GameplayStatics.BreakHitResult` _outhit))
  (if _bblockinghit
    (bind _output_get (set `self.Impact Point` _impactpoint))
    (set `SpringArmComponent.TargetArmLength` (`KismetMathLibrary.FInterpTo` (`SpringArmComponent.TargetArmLength` (`self.SpringArmComp`)) (- (`KismetMathLibrary.Vector_Distance` _output_get (`SceneComponent.K2_GetComponentLocation` (`self.SpringArmComp`))) (`self.Radius`)) (`GameplayStatics.GetWorldDeltaSeconds`) 3.0) (`self.SpringArmComp`))
    (elif (not (`KismetMathLibrary.NearlyEqual_FloatFloat` (`SpringArmComponent.TargetArmLength` (`self.SpringArmComp`)) (`self.DefaultSpringArmLength`) 1.0))
      (set `SpringArmComponent.TargetArmLength` (`KismetMathLibrary.FInterpTo` (`SpringArmComponent.TargetArmLength` (`self.SpringArmComp`)) (`self.DefaultSpringArmLength`) (`GameplayStatics.GetWorldDeltaSeconds`) 3.0) (`self.SpringArmComp`)))))

(event `Key|E`
  (params (Key :type "Key Structure"))
  ;[1 1 1] Event Trigger
  (:`Pressed`
    (`self.Grab Server`)))

(event `Grab Server`
  ;[1 1 1] Event Trigger
  (`self.Grab Client`))

(event `ObjectDroppedServer`
  (params (GrabObject :type "/Game/Kyoulee/BluePrints/Replicate/BP_GrabBase Object Reference") (PhysicsHandle :type "PhysicsHandleComponent Object Reference"))
  ;[1 1 1] DropObject
  (`/Game/Kyoulee/BluePrints/Replicate/BP_GrabBase.Update Physics Replicates` GrabObject true)
  (`self.ObjectDroppedMulticast` PhysicsHandle))

(event `ObjectGrabbedServer`
  (params (GrabObject :type "/Game/Kyoulee/BluePrints/Replicate/BP_GrabBase Object Reference") (PhysicsHandle :type "PhysicsHandleComponent Object Reference") (`Hit Component` :type "PrimitiveComponent Object Reference") (Location :type "Vector Structure"))
  ;[1 1 1] grab objects
  (`/Game/Kyoulee/BluePrints/Replicate/BP_GrabBase.Update Physics Replicates` GrabObject false)
  (`self.ObjectGrabbedMuticast` PhysicsHandle `Hit Component` Location))

(event `SetNewLocationServer`
  (params (PhysicsHandle :type "PhysicsHandleComponent Object Reference") (NewLocation :type "Vector Structure") (NewRotation :type "Rotator Structure"))
  ;[1 1 1] SetLocation
  (`self.SetNewLocationMulticast` PhysicsHandle NewLocation NewRotation)
  (`self.SetNewLocationClient` PhysicsHandle NewLocation NewRotation))

(event `ObjectDroppedMulticast`
  (params (PhysicsHandle :type "PhysicsHandleComponent Object Reference"))
  ;[1 1 1] DropObject
  (`PhysicsHandleComponent.ReleaseComponent` PhysicsHandle))

(event `ObjectGrabbedMuticast`
  (params (`Physics Handle` :type "PhysicsHandleComponent Object Reference") (`Hit Component` :type "PrimitiveComponent Object Reference") (Location :type "Vector Structure"))
  ;[1 1 1] grab objects
  (`PhysicsHandleComponent.GrabComponentAtLocation` `Physics Handle` `Hit Component` "None" Location))

(event `SetNewLocationMulticast`
  (params (PhysicsHandle :type "PhysicsHandleComponent Object Reference") (NewLocation :type "Vector Structure") (NewRotation :type "Rotator Structure"))
  ;[1 1 1] SetLocation
  (`PhysicsHandleComponent.SetTargetLocationAndRotation` PhysicsHandle NewLocation NewRotation))

(event `SetNewLocationClient`
  (params (PhysicsHandle :type "PhysicsHandleComponent Object Reference") (NewLocation :type "Vector Structure") (NewRotation :type "Rotator Structure"))
  ;[1 1 1] SetLocation
  (`PhysicsHandleComponent.SetTargetLocationAndRotation` PhysicsHandle NewLocation NewRotation))

(event `Grab Client`
  (bind _capsulecomponent (`self.CapsuleComponent`))
  ;[1 1 1] Grab Action
  (if (`self.Is Grabing Object`)
    (`self.ObjectDroppedServer` (`self.As BP Grab Base`) (`self.PhysicsHandle`))
    (set `self.Is Grabing Object` false)
    (else
      (bind (_outhit _returnvalue) (`KismetSystemLibrary.LineTraceSingleForObjects` (+ (`SceneComponent.K2_GetComponentLocation` _capsulecomponent) (* (`KismetMathLibrary.GetForwardVector` (`SceneComponent.K2_GetComponentRotation` _capsulecomponent)) 10.0)) (+ (`SceneComponent.K2_GetComponentLocation` _capsulecomponent) (* (`KismetMathLibrary.GetForwardVector` (`SceneComponent.K2_GetComponentRotation` (`self.CameraComp`))) 1000.0)) (`|MakeArray` "ObjectTypeQuery4" :!type "EObjectTypeQuery Enum")))
      (if _returnvalue
        (bind (_bblockinghit _binitialoverlap _time _distance _location _impactpoint _normal _impactnormal _physmat _hitactor _hitcomponent) (`GameplayStatics.BreakHitResult` _outhit))
        (bind _asbp_grab_base (cast `/Game/Kyoulee/BluePrints/Replicate/BP_GrabBase` _hitactor))
        (bind _output_get (set `self.As BP Grab Base` _asbp_grab_base))
        (`self.ObjectGrabbedServer` _output_get (`self.PhysicsHandle`) _hitcomponent (`SceneComponent.K2_GetComponentLocation` _hitcomponent))
        (set `self.Is Grabing Object` true)))))

(event `self.ReceiveTick`
  (params (DeltaSeconds :type "Float (single-precision)"))
  (bind _returnvalue (`SceneComponent.K2_GetComponentRotation` (`self.CameraComp`)))
  ;[1 1 1] Tick Update Grap Component
  (`|ExecutionSequence`
    (:`then_0`
      (if (`self.Is Grabing Object`)
        (`self.SetNewLocationServer` (`self.PhysicsHandle`) (+ (`SceneComponent.K2_GetComponentLocation` (`self.CapsuleComponent`)) (* (`KismetMathLibrary.GetForwardVector` _returnvalue) 150.0)) _returnvalue)))
    (:`then_1`
      (`self.Canmeracolision`))))

(fn `ChangeSkeletalMesh`
  (bind _asbp_character_game_instance (cast `/Game/Kyoulee/WidGets/Character/BP_CharacterGameInstance` (`GameplayStatics.GetGameInstance`)))
  (`SkeletalMeshComponent.SetSkeletalMeshAsset` (`self.Mesh`) (`SkeletalMeshComponent.SkeletalMeshAsset` (`/Game/Kyoulee/WidGets/Character/BP_CharacterGameInstance.CharacterMesh` _asbp_character_game_instance))))

(fn `FirstPersonViewFunc`
  (`SceneComponent.K2_SetRelativeLocation` (`self.CameraComp`) (`SceneComponent.RelativeLocation` (`self.firstpersonposision`)) false false))

(fn `get interp Speed`
  (returns (NewParam :type "Float (double-precision)"))
  (bind _interpspeed (`self.interpspeed`))
  (bind _output_get (set `self.interpspeed` (`KismetMathLibrary.MapRangeClamped` (`KismetMathLibrary.Vector_Distance` (`SceneComponent.K2_GetComponentLocation` (`self.CameraComp`)) (`self.Impact Point`)) 0.0 (`self.DefaultSpringArmLength`) _interpspeed (* _interpspeed 10.0))))
  (return _output_get))

(fn `ThirdPersonViewFunc`
  (`SceneComponent.K2_SetRelativeLocation` (`self.CameraComp`) (`SceneComponent.RelativeLocation` (`self.thirdpersonposision`)) false false))

(fn `UserConstructionScript`)