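; BP_Overlap is a trigger actor that shows the WBP_Earth widget and mouse cursor when overlapped, without checking which actor entered.
; Begin overlap, or CustomEvent, loops over every BP_BaseCharacter, enabling player 0's cursor and adding a new widget per character if that controller is local.
; End overlap removes all widgets and hides the cursor.
; A UI-only input mode call exists but is unconnected.
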(event `self.ReceiveActorBeginOverlap`
  (params (OtherActor :type "Actor Object Reference"))
  (bind _returnvalue (`GameplayStatics.GetPlayerController` 0))
  (bind _outactors (`GameplayStatics.GetAllActorsOfClass` "/Game/GW/BluePrint/BP_BaseCharacter.BP_BaseCharacter_C" :!label _label))
  (for _ _outactors
    (set `PlayerController.bShowMouseCursor` true _returnvalue)
    (if (`Controller.IsLocalController` _returnvalue)
      (bind _returnvalue_2 (`|CreateWidget` "/Game/GW/UI/WBP_Earth.WBP_Earth_C"))
      (`UserWidget.AddToViewport` _returnvalue_2 0))))

(event `CustomEvent`
  (goto _label))

(event `OnActorBeginOverlap_Event`
  (params (OverlappedActor :type "Actor Object Reference") (OtherActor :type "Actor Object Reference")))

(event `self.ReceiveActorEndOverlap`
  (params (OtherActor :type "Actor Object Reference"))
  (`WidgetLayoutLibrary.RemoveAllWidgets`)
  (set `PlayerController.bShowMouseCursor` false (`GameplayStatics.GetPlayerController` 0)))

(fn `UserConstructionScript`)