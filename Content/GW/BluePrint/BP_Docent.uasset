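; BP_Docent is a docent actor that turns to face the player character while the player is inside its Box.
; On BeginPlay it spawns a BP_HttpActor and caches the player as BP_BaseCharacter.
; Self-calling events with short Delays, used instead of Tick, poll the Box overlap and interpolate yaw toward the player.
; The talk event only casts the HTTP actor reference and does nothing further.
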(event `self.ReceiveBeginPlay`
  (`|ExecutionSequence`
    (:`then_0`
      (bind _returnvalue (`|SpawnActorFromClass` "/Game/GW/BluePrint/BP_HttpActor.BP_HttpActor_C" (`self.Spawn Transform`) "Undefined" "MultiplyWithRoot" null null))
      (set `self.httpactor` _returnvalue))
    (:`then_1`
      (bind _asbp_base_character (cast `/Game/GW/BluePrint/BP_BaseCharacter` (`GameplayStatics.GetPlayerCharacter` 0)))
      (set `self.As BP Base Character` _asbp_base_character)
      (`self.ShouldRotateFunc`))))

(event `talk`
  (cast `HttpActor` (`self.httpactor`)))

(event `FaceCharacter`
  (bind (_returnvalue_roll _returnvalue_pitch _returnvalue_yaw) (`KismetMathLibrary.BreakRotator` (`KismetMathLibrary.RInterpTo` (`self.K2_GetActorRotation`) (`KismetMathLibrary.FindLookAtRotation` (`self.K2_GetActorLocation`) (`self.K2_GetActorLocation` (`self.As BP Base Character`))) (`GameplayStatics.GetWorldDeltaSeconds`) 5.0)))
  (if (`self.ShouldRotate`)
    (`self.K2_SetActorRotation` (`KismetMathLibrary.MakeRotator` 0.0 0.0 _returnvalue_yaw))
    (`KismetSystemLibrary.Delay` 0.01)
    (`self.FaceCharacter`)
    (else
      (`self.ShouldRotateFunc`))))

(event `ShouldRotateFunc`
  (if (`PrimitiveComponent.IsOverlappingActor` (`self.Box`) (`self.As BP Base Character`))
    (set `self.ShouldRotate` true)
    (`self.FaceCharacter`)
    (else
      (set `self.ShouldRotate` false)))
  (`KismetSystemLibrary.Delay` 0.01)
  (`self.ShouldRotateFunc`))

(fn `UserConstructionScript`)