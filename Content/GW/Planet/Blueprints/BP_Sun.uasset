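; BP_Sun is a sun actor that orbits a center point, following an optional center actor if it moves.
; Each tick it rotates its offset from the previous center around an axis at a set speed, then re-anchors it on the current center.
; Before each step, a double cross product re-orthogonalizes the axis against that offset, keeping the orbit a great circle around the center.
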(event `OrthogonalizeAxis`
  (bind _returnvalue (- (`self.K2_GetActorLocation`) (`self.OldCenterLocation`)))
  (set `self.Axis` (`KismetMathLibrary.Normal` (`KismetMathLibrary.Cross_VectorVector` _returnvalue (`KismetMathLibrary.Cross_VectorVector` (`self.Axis`) _returnvalue)))))

(event `self.ReceiveBeginPlay`
  (`|ExecutionSequence`
    (:`then_0`
      (bind _centeractor (`self.CenterActor`)
        (:`then`
          (set `self.CenterLocation` (`self.K2_GetActorLocation` _centeractor)))
        (:`else`)))
    (:`then_1`
      (set `self.OldCenterLocation` (`self.CenterLocation`)))))

(event `self.ReceiveTick`
  (params (DeltaSeconds :type "Float (single-precision)"))
  (`|ExecutionSequence`
    (:`then_0`
      (bind _centeractor (`self.CenterActor`)
        (:`then`
          (set `self.CenterLocation` (`self.K2_GetActorLocation` _centeractor)))
        (:`else`)))
    (:`then_1`
      (`self.OrthogonalizeAxis`)
      (`self.K2_SetActorLocation` (+ (`KismetMathLibrary.RotateAngleAxis` (- (`self.K2_GetActorLocation`) (`self.OldCenterLocation`)) (* DeltaSeconds (`self.speed`)) (`self.Axis`)) (`self.CenterLocation`)))
      (set `self.OldCenterLocation` (`self.CenterLocation`)))))

(fn `UserConstructionScript`)